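; Third-person shooter character Blueprint that handles firing animations and the aim camera zoom.
; BeginPlay binds to shoot, start-aim and stop-aim events; shooting animates the weapon and plays an ironsights or hip-fire montage based on IsAiming.
; Aim events stop the opposing zoom timeline and restart their own.
; Both timelines feed SetCameraOffset, which remaps zoom from the camera boom's current socket X offset toward a target.
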(event `self.ReceiveBeginPlay`
  (`|ExecutionSequence`
    (:`then_0`
      (add `self.OnShoot` (delegate `OnShoot_Event`)))
    (:`then_1`
      (add `self.FOnStartAim` (delegate `FOnStartAim_Event`)))
    (:`then_2`
      (add `self.FOnStopAim` (delegate `FOnStopAim_Event`)))))

(event `OnShoot_Event`
  (`SkeletalMeshComponent.PlayAnimation` (`self.Weapon`) "/Game/MilitaryWeapDark/Weapons/Anims/Fire_Rifle_W.Fire_Rifle_W" false)
  (if (`self.bIsAiming`)
    (`|PlayMontage` (`self.Mesh`) "/Game/AnimStarterPack/Retargeted_UE5_Anims/Fire_Rifle_Ironsights_Montage.Fire_Rifle_Ironsights_Montage")
    (else
      (`|PlayMontage` (`self.Mesh`) "/Game/AnimStarterPack/Retargeted_UE5_Anims/Fire_Rifle_Hip_Montage.Fire_Rifle_Hip_Montage"))))

(event `FOnStartAim_Event`
  (`|ExecutionSequence`
    (:`then_0`
      (bind (_direction _zoom) (`Timeline|WeaponZoomOut` :!via `Stop` :!label _label)
        (:`Update`
          (`self.SetCameraOffset` _zoom 100.0))))
    (:`then_1`
      (bind (_direction_2 _zoom_2) (`Timeline|WeaponZoomIn` :!via `PlayFromStart` :!label _label_2)
        (:`Update`
          (`self.SetCameraOffset` _zoom_2 0.0 100.0 150.0))))))

(event `FOnStopAim_Event`
  (`|ExecutionSequence`
    (:`then_0`
      (goto _label_2 :!via `Stop`))
    (:`then_1`
      (goto _label :!via `PlayFromStart`))))

(fn `OnRep_NewVar`)

(fn `SetCameraOffset`
  (params (ZoomAmount :type "Float (double-precision)") (InRangeA :type "Float (double-precision)") (InRangeB :type "Float (double-precision)") (TargetXOffset :type "Float (double-precision)"))
  (bind _cameraboom (`self.CameraBoom`))
  (bind _socketoffset_x (`KismetMathLibrary.BreakVector` (`SpringArmComponent.SocketOffset` (`self.CameraBoom`))))
  (bind (_socketoffset_x_2 _socketoffset_y _socketoffset_z) (`KismetMathLibrary.BreakVector` (`SpringArmComponent.SocketOffset` _cameraboom)))
  (set `SpringArmComponent.SocketOffset` (`KismetMathLibrary.MakeVector` (`KismetMathLibrary.MapRangeClamped` ZoomAmount InRangeA InRangeB _socketoffset_x TargetXOffset) _socketoffset_y _socketoffset_z) _cameraboom))

(fn `UserConstructionScript`)